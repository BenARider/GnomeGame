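; Gnome pawn with twin-stick controls that moves on physics and fires a charged rod projectile.
; Each Tick, left-stick force pushes the speed-capped capsule, swapping physical materials for moving or idle, while the right stick smoothly turns the body.
; A speed-driven phase flip rocks the body side to side as a procedural waddle.
; Holding Space or the axis key blocks movement, pitches the body and builds charge; release spawns a projectile with charge-scaled speed.
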(event EventTick
  (params (DeltaSeconds :type Float%20%28single-precision%29))
  (bind _returnvalue (Math|Vector|MakeVector 1.0 0.0 0.0))
  (bind _returnvalue_2 (Class|Actor|GetInputAxisKeyValue))
  (bind _returnvalue_3 (Input|AxisValues|GetMoveForward))
  (bind _returnvalue_4 (Input|AxisValues|GetMoveRight))
  (bind _returnvalue_5 (Input|AxisValues|GetFireForward))
  (bind _returnvalue_6 (Input|AxisValues|GetFireRight))
  (bind _maxcharge (Variables|Default|GetMaxCharge))
  (bind _spacedown (Variables|Default|GetSpaceDown))
  (bind _capsule (Variables|Default|GetCapsule))
  (bind _movemaxspeed (Variables|Default|GetMoveMaxSpeed))
  (bind _capsule_2 (Variables|Default|GetCapsule))
  (bind _body (Variables|Default|GetBody))
  (bind _capsule_3 (Variables|Default|GetCapsule))
  (bind _body_2 (Variables|Default|GetBody))
  (bind _capsule_4 (Variables|Default|GetCapsule))
  (bind _returnvalue_7 (Math|Float|Truncate _returnvalue_2))
  (bind _returnvalue_8 (Math|Conversions|ToInteger(Boolean) _spacedown))
  (bind _returnvalue_9 (Math|Vector|MakeVector _returnvalue_3 _returnvalue_4 0.0))
  (bind _returnvalue_10 (Transformation|GetComponentVelocity _capsule))
  (bind _returnvalue_11 (Transformation|GetComponentVelocity _capsule_4))
  (bind _returnvalue_12 (Transformation|GetComponentVelocity _capsule_2))
  (bind (_x _y) (Math|Vector|BreakVector _returnvalue_10))
  (bind _returnvalue_13 (Math|Vector|VectorLength _returnvalue_12))
  (bind _returnvalue_14 (Math|Vector|ClampVectorSize _returnvalue_11 0.0 _movemaxspeed))
  (bind _returnvalue_15 (Class|KismetMathLibrary|OrIntInt _returnvalue_7 _returnvalue_8))
  (bind _returnvalue_16 (/ _returnvalue_13 5.0))
  (bind _returnvalue_17 (Math|Conversions|ToFloat(Integer) _returnvalue_15))
  (bind (_x_2 _y_2) (Math|Vector|BreakVector _returnvalue_14))
  (bind _returnvalue_18 (> _returnvalue_17 0.1))
  (if _returnvalue_18
    (Variables|Default|SetCanControl false)
    (else
      (Variables|Default|SetCanControl true)))
  (Utilities|FlowControl|Sequence
    (:then_0
      (if (Variables|Default|GetCanControl)
        ;[1 1 1] Physics movement from left stick
        (if (> (Math|Vector|VectorLengthXY _returnvalue_9) 0.1)
          (Class|PrimitiveComponent|SetPhysMaterialOverride _capsule_3 "/Game/Assets/Blueprints/GnomeMoveMat.GnomeMoveMat")
          (else
            (Class|PrimitiveComponent|SetPhysMaterialOverride _capsule_3 "/Game/Assets/Blueprints/GnomeStaticMat.GnomeStaticMat")))
        (Physics|AddForce (Variables|Default|GetCapsule) (* (* _returnvalue_9 (Variables|Default|GetMoveImpulse)) DeltaSeconds) "None" true)
        (Physics|SetPhysicsLinearVelocity (Variables|Default|GetCapsule) (Math|Vector|MakeVector _x_2 _y_2 (.Z (Math|Vector|BreakVector _returnvalue_11))) false "None")
        ;[1 1 1] Set Animation state
        (if (< (Math|Vector|VectorLengthXY (Math|Vector|MakeVector _x _y 0.0)) 5.0)
          (Variables|Default|SetMovePhase 0)
          (elif (== (Variables|Default|GetMovePhase) 0)
            (Variables|Default|SetMovePhase 1)))
        (switch int (Variables|Default|GetMovePhase)
          (:0
            (Variables|Default|SetMoveVal (/ (Variables|Default|GetMoveVal) 1.1)))
          (:1
            (bind _output_get (Variables|Default|SetMoveVal (+ (Variables|Default|GetMoveVal) (* _returnvalue_16 DeltaSeconds))))
            (if (> _output_get 2.0)
              (Variables|Default|SetMovePhase 2)))
          (:2
            (bind _output_get_2 (Variables|Default|SetMoveVal (+ (Variables|Default|GetMoveVal) (* (* _returnvalue_16 -1.0) DeltaSeconds))))
            (if (< _output_get_2 -2.0)
              (Variables|Default|SetMovePhase 1))))
        (else
          (Variables|Default|SetMovePhase 0)
          (Class|PrimitiveComponent|SetPhysMaterialOverride (Variables|Default|GetCapsule)))))
    (:then_1
      ;[1 1 1] Rotate based on right stick
      (if (and (== _returnvalue_5 0.0) (== _returnvalue_6 0.0))
        (Transformation|SetWorldRotation _body (Variables|Default|GetworldRotDir) false false)
        (else
          (Transformation|SetWorldRotation _body (Math|Interpolation|RInterpTo (Variables|Default|GetworldRotDir) (Math|Conversions|RotationFromXVector (Math|Vector|MakeVector _returnvalue_5 _returnvalue_6 0.0)) DeltaSeconds (Variables|Default|GetRotateSpeed)) false false)
          (Variables|Default|SetworldRotDir (Transformation|GetWorldRotation _body)))))
    (:then_2
      ;[1 1 1] Rotate based on animation state
      (switch int (Variables|Default|GetMovePhase)
        (:1
          (Transformation|AddLocalRotation _body_2 (Math|Vector|RotatorfromAxisandAngle _returnvalue 1e+01) false false))
        (:2
          (Transformation|AddLocalRotation _body_2 (Math|Vector|RotatorfromAxisandAngle _returnvalue -1e+01) false false))))
    (:then_3
      ;[1 1 1] Rod Animation
      (if _returnvalue_18
        (Utilities|FlowControl|Sequence
          (:then_0
            (Transformation|AddLocalRotation (Variables|Default|GetBody) (Math|Vector|RotatorfromAxisandAngle (Math|Vector|MakeVector 0.0 1.0 0.0) -2e+01) false false))
          (:then_1
            ;[1 1 1] Rod Charge and Throw
            (bind _output_get_3 (Variables|Default|SetChargeVal (+ (Variables|Default|GetChargeVal) 0.5))) ; While space is held, increase charge val
            (if (>= _output_get_3 _maxcharge)
              (Variables|Default|SetChargeVal _maxcharge))
            (Development|PrintString (Utilities|String|ToString(Float) _output_get_3))))
        (elif (> (Variables|Default|GetChargeVal) 0.0) ; If charge button is let go, and chargeval has a value, reset charge value and fire
          (Game|SpawnActorfromClass "/Game/Assets/Blueprints/Projectile.Projectile_C" (Math|Transform|MakeTransform (Transformation|GetWorldLocation (Variables|Default|GetProjectileFirePoint)) (Variables|Default|GetworldRotDir) "0.400000,0.400000,0.400000") "Undefined" 0 (* (Variables|Default|GetChargeVal) 1e+01) 0)
          (Variables|Default|SetChargeVal 0.0))))))

(event Input|KeyboardEvents|SpaceBar
  (params (Key :type Key%20Structure))
  (:Pressed
    (Variables|Default|SetSpaceDown true))
  (:Released
    (Variables|Default|SetSpaceDown false)))

(fn ConstructionScript)