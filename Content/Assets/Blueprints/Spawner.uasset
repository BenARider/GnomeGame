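; Spawner Blueprint that sizes a Players array when play begins; it does not yet spawn anything.
; BeginPlay runs a counter-driven while loop that adds an unspecified element until the counter reaches PlayerCount, then prints the array length.
; Tick is disabled and the construction script is empty.
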(event EventBeginPlay
  (while (< (Variables|Default|GetaddToPlayerArrayCounter) (Variables|Default|GetplayerCount))
    (Utilities|Array|Add (Variables|Default|GetPlayers) 0)
    (Variables|Default|SetaddToPlayerArrayCounter (+ (Variables|Default|GetaddToPlayerArrayCounter) 1)))
  (Development|PrintString (Utilities|String|ToString(Integer) (Utilities|Array|Length (Variables|Default|GetPlayers)))))

(event EventTick
  (params (DeltaSeconds :type Float%20%28single-precision%29)))

(fn ConstructionScript)