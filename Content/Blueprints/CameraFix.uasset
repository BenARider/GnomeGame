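; Shared multiplayer camera actor that frames up to four Gnome players and becomes the view target for all player controllers.
; Setup gathers all Gnomes under GM_RR, or active, living players from KingOfTheGarden, into PlayerReference and Gnome slots.
; A fast looping timer runs a per-player-count function that interpolates toward the gnomes' average location plus an offset.
; Spring arm length follows the largest pairwise gnome distance, clamped, or uses the minimum for one player.
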(event Custom|UpdateCamera
  (switch int (Utilities|Array|Length (Variables|Default|GetPlayerReference))
    (:1
      (CallFunction|1Player))
    (:2
      (CallFunction|2Player))
    (:3
      (CallFunction|3Player))
    (:4
      (CallFunction|4Player))))

(event EventBeginPlay
  (Utilities|FlowControl|Delay 0.01)
  (CallFunction|Setup)
  (Utilities|Time|SetTimerbyFunctionName 0 "UpdateCamera" 0.001 true))

(fn ConstructionScript)

(fn Setup
  (bind _returnvalue (Game|GetGameMode))
  (bind _asgm_rr (Utilities|Casting|CastToGM_RR _returnvalue)
    (:then
      (bind _output_get (Variables|Default|SetGM_RR _asgm_rr))
      (bind _outactors (Actor|GetAllActorsOfClass "/Game/Blueprints/Gnome.Gnome_C"))
      (Variables|/Game/Blueprints/GM_RR.GM_RR_C|SetRemainingPlayers _output_get _outactors)
      (Variables|Default|SetPlayerReference _outactors))
    (:CastFailed
      (bind _asking_of_the_garden (Utilities|Casting|CastToKingOfTheGarden _returnvalue))
      (Utilities|Array|Clear (Variables|Default|GetPlayerReference))
      (if (Variables|/Game/KingOfTheGarden/KingOfTheGarden.KingOfTheGarden_C|GetP1Active _asking_of_the_garden)
        (if (Utilities|Array|Get(acopy) (Variables|/Game/KingOfTheGarden/KingOfTheGarden.KingOfTheGarden_C|GetIsDead _asking_of_the_garden))
          _
          (else
            (Utilities|Array|Add (Variables|Default|GetPlayerReference) (Utilities|Array|Get(acopy) (Variables|/Game/KingOfTheGarden/KingOfTheGarden.KingOfTheGarden_C|GetPlayers _asking_of_the_garden))))))
      (if (Variables|/Game/KingOfTheGarden/KingOfTheGarden.KingOfTheGarden_C|GetP2Active _asking_of_the_garden)
        (if (Utilities|Array|Get(acopy) (Variables|/Game/KingOfTheGarden/KingOfTheGarden.KingOfTheGarden_C|GetIsDead _asking_of_the_garden) 1)
          _
          (else
            (Utilities|Array|Add (Variables|Default|GetPlayerReference) (Utilities|Array|Get(acopy) (Variables|/Game/KingOfTheGarden/KingOfTheGarden.KingOfTheGarden_C|GetPlayers _asking_of_the_garden) 1)))))
      (if (Variables|/Game/KingOfTheGarden/KingOfTheGarden.KingOfTheGarden_C|GetP3Active _asking_of_the_garden)
        (if (Utilities|Array|Get(acopy) (Variables|/Game/KingOfTheGarden/KingOfTheGarden.KingOfTheGarden_C|GetIsDead _asking_of_the_garden) 2)
          _
          (else
            (Utilities|Array|Add (Variables|Default|GetPlayerReference) (Utilities|Array|Get(acopy) (Variables|/Game/KingOfTheGarden/KingOfTheGarden.KingOfTheGarden_C|GetPlayers _asking_of_the_garden) 2)))))
      (if (Variables|/Game/KingOfTheGarden/KingOfTheGarden.KingOfTheGarden_C|GetP4Active _asking_of_the_garden)
        (if (Utilities|Array|Get(acopy) (Variables|/Game/KingOfTheGarden/KingOfTheGarden.KingOfTheGarden_C|GetIsDead _asking_of_the_garden) 3)
          _
          (else
            (Utilities|Array|Add (Variables|Default|GetPlayerReference) (Utilities|Array|Get(acopy) (Variables|/Game/KingOfTheGarden/KingOfTheGarden.KingOfTheGarden_C|GetPlayers _asking_of_the_garden) 3)))))))
  (bind _outactors_2 (Actor|GetAllActorsOfClass "/Script/Engine.PlayerController"))
  (Game|Player|SetViewTargetwithBlend _outactors_2 self 0.0 "VTBlend_Linear" 0.0 false)
  (for (_array_element _array_index) (Variables|Default|GetPlayerReference)
    (switch int _array_index
      (:0
        (Variables|Default|SetGnome1 _array_element))
      (:1
        (Variables|Default|SetGnome2 _array_element))
      (:2
        (Variables|Default|SetGnome3 _array_element))
      (:3
        (Variables|Default|SetGnome4 _array_element)))))

(fn 4Player
  (bind _gnome1 (Variables|Default|GetGnome1))
  (bind _gnome2 (Variables|Default|GetGnome2))
  (bind _gnome3 (Variables|Default|GetGnome3))
  (bind _gnome4 (Variables|Default|GetGnome4))
  (Variables|/Script/Engine.SpringArmComponent|SetTargetArmLength (Variables|Default|GetSpringArm) (Math|Float|Clamp(Float) (.MaxValue (Math|Float|MaxOfFloatArray (Utilities|Array|MakeArray (Transformation|GetDistanceTo _gnome1 _gnome2) (Transformation|GetDistanceTo _gnome1 _gnome3) (Transformation|GetDistanceTo _gnome1 _gnome4) (Transformation|GetDistanceTo _gnome2 _gnome3) (Transformation|GetDistanceTo _gnome2 _gnome4) (Transformation|GetDistanceTo _gnome4 _gnome3)))) (Variables|Default|GetminArm) (Variables|Default|GetmaxArm)))
  (bind _output_get (Variables|Default|SetTargetPos (+ (/ (+ (Transformation|GetActorLocation (Variables|Default|GetGnome1)) (Transformation|GetActorLocation (Variables|Default|GetGnome2)) (Transformation|GetActorLocation (Variables|Default|GetGnome3)) (Transformation|GetActorLocation (Variables|Default|GetGnome4))) (Math|Conversions|ToFloat(Integer) (Utilities|Array|Length (Variables|Default|GetPlayerReference)))) (Variables|Default|GetOffset))))
  (Transformation|SetActorLocation (Math|Interpolation|VInterpTo (Variables|Default|GetLastPos) _output_get (Utilities|Time|GetWorldDeltaSeconds) 1e+01) false false)
  (Variables|Default|SetLastPos (Transformation|GetActorLocation)))

(fn 3Player
  (bind _gnome1 (Variables|Default|GetGnome1))
  (bind _gnome2 (Variables|Default|GetGnome2))
  (bind _gnome3 (Variables|Default|GetGnome3))
  (Variables|/Script/Engine.SpringArmComponent|SetTargetArmLength (Variables|Default|GetSpringArm) (Math|Float|Clamp(Float) (.MaxValue (Math|Float|MaxOfFloatArray (Utilities|Array|MakeArray (Transformation|GetDistanceTo _gnome1 _gnome2) (Transformation|GetDistanceTo _gnome1 _gnome3) (Transformation|GetDistanceTo _gnome2 _gnome3)))) (Variables|Default|GetminArm) (Variables|Default|GetmaxArm)))
  (bind _output_get (Variables|Default|SetTargetPos (+ (/ (+ (Transformation|GetActorLocation (Variables|Default|GetGnome1)) (Transformation|GetActorLocation (Variables|Default|GetGnome2)) (Transformation|GetActorLocation (Variables|Default|GetGnome3))) (Math|Conversions|ToFloat(Integer) (Utilities|Array|Length (Variables|Default|GetPlayerReference)))) (Variables|Default|GetOffset))))
  (Transformation|SetActorLocation (Math|Interpolation|VInterpTo (Variables|Default|GetLastPos) _output_get (Utilities|Time|GetWorldDeltaSeconds) 1e+01) false false)
  (Variables|Default|SetLastPos (Transformation|GetActorLocation)))

(fn 2Player
  (Variables|/Script/Engine.SpringArmComponent|SetTargetArmLength (Variables|Default|GetSpringArm) (Math|Float|Clamp(Float) (Transformation|GetDistanceTo (Variables|Default|GetGnome1) (Variables|Default|GetGnome2)) (Variables|Default|GetminArm) (Variables|Default|GetmaxArm)))
  (bind _output_get (Variables|Default|SetTargetPos (+ (/ (+ (Transformation|GetActorLocation (Variables|Default|GetGnome1)) (Transformation|GetActorLocation (Variables|Default|GetGnome2))) (Math|Conversions|ToFloat(Integer) (Utilities|Array|Length (Variables|Default|GetPlayerReference)))) (Variables|Default|GetOffset))))
  (Transformation|SetActorLocation (Math|Interpolation|VInterpTo (Variables|Default|GetLastPos) _output_get (Utilities|Time|GetWorldDeltaSeconds) 1e+01) false false)
  (Variables|Default|SetLastPos (Transformation|GetActorLocation)))

(fn 1Player
  (Variables|/Script/Engine.SpringArmComponent|SetTargetArmLength (Variables|Default|GetSpringArm) (Variables|Default|GetminArm))
  (bind _output_get (Variables|Default|SetTargetPos (+ (Transformation|GetActorLocation (Variables|Default|GetGnome1)) (Variables|Default|GetOffset))))
  (Transformation|SetActorLocation (Math|Interpolation|VInterpTo (Variables|Default|GetLastPos) _output_get (Utilities|Time|GetWorldDeltaSeconds) 1e+01) false false)
  (Variables|Default|SetLastPos (Transformation|GetActorLocation)))