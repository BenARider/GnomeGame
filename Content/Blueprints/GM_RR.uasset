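; GM_RR is a game mode Blueprint that gathers player starts and runs a minutes-and-seconds countdown.
; BeginPlay caches all PlayerStart actors, then calls SpawnPlayers, whose loop over the player count has an empty body.
; Disconnected logic would create local players and possess Gnome pawns at starts tagged by index.
; Tick uses a one-second Delay to decrement the timer, with no stop at zero.
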(event EventBeginPlay
  (CallFunction|GetPlayerStartPoints)
  (CallFunction|SpawnPlayers))

(event EventTick
  (params (DeltaSeconds :type Float%20%28single-precision%29))
  (Utilities|FlowControl|Delay 1.0)
  (Variables|Default|SetSeconds (- (Variables|Default|GetSeconds) 1))
  (if (< (Variables|Default|GetSeconds) 0)
    (Variables|Default|SetMinutes (- (Variables|Default|GetMinutes) 1))
    (Variables|Default|SetSeconds 59)))

(fn ConstructionScript)

(fn GetPlayerStartPoints
  (bind _outactors (Actor|GetAllActorsOfClass "/Script/Engine.PlayerStart"))
  (Variables|Default|SetPlayer%20start%20array _outactors))

(fn SpawnPlayers
  (for _index (range 0 (- (Variables|Default|GetMaxPlayerCount) 1))
    _))