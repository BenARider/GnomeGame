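; Flaming Boots item Blueprint, a pickup that grants the boots to the player who collects it.
; Its Pickup override checks the player's ItemMap, then marks the boots as owned, notifies the player with the item ID and runs the parent pickup logic.
; If the player already owns the boots, it skips the pickup and prints a debug message.
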(event EventBeginPlay
  (|CallParentFunction) ; This node is disabled and will not be called.\nDrag off pins to build functionality.
)

(event Collision|EventActorBeginOverlap
  (params (OtherActor :type Actor%20Object%20Reference))
  (|CallParentFunction OtherActor) ; This node is disabled and will not be called.\nDrag off pins to build functionality.
)

(event EventTick
  (params (DeltaSeconds :type Float%20%28single-precision%29))
  (|CallParentFunction DeltaSeconds) ; This node is disabled and will not be called.\nDrag off pins to build functionality.
)

(fn ConstructionScript
  (|CallParentFunction))

(fn Pickup
  (params (PlayerWhoCollectedItem :type Gnome%20Object%20Reference%20%28by%20ref%29))
  ;[1 1 1] If the player already has the item, don't pick it up again
  (if (Math|Boolean|Equal(Boolean) (.Value (Utilities|Map|Find (Variables|/Game/Blueprints/Gnome.Gnome_C|GetItemMap PlayerWhoCollectedItem) "FlamingBoots_C")) false)
    (Utilities|Map|Add (Variables|/Game/Blueprints/Gnome.Gnome_C|GetItemMap PlayerWhoCollectedItem) "FlamingBoots_C" true)
    (Default|ItemPickedUp PlayerWhoCollectedItem (Variables|Default|GetItemID))
    (bind _unreal_needs_an_output_for_an_overriden_function_to_count_as_a_function_instead_of_an_event (|CallParentFunction PlayerWhoCollectedItem))
    (return _unreal_needs_an_output_for_an_overriden_function_to_count_as_a_function_instead_of_an_event)
    (else
      (Development|PrintString "Already has flaming boots"))))