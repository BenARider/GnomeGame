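; HealthPack is a pickup item Blueprint that heals the player who collects it.
; Its Pickup override spawns a particle effect at the MFish component's location, calls Heal on the collector with HealVal and prints a debug message.
; It then calls the parent Pickup, which destroys the actor; the event graph holds only disabled default events.
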(event EventBeginPlay
  (|CallParentFunction) ; This node is disabled and will not be called.\nDrag off pins to build functionality.
)

(event Collision|EventActorBeginOverlap
  (params (OtherActor :type Actor%20Object%20Reference))
  (|CallParentFunction OtherActor) ; This node is disabled and will not be called.\nDrag off pins to build functionality.
)

(event EventTick
  (params (DeltaSeconds :type Float%20%28single-precision%29))
  (|CallParentFunction DeltaSeconds) ; This node is disabled and will not be called.\nDrag off pins to build functionality.
)

(fn ConstructionScript
  (|CallParentFunction))

(fn Pickup
  (params (PlayerWhoCollectedItem :type Gnome%20Object%20Reference%20%28by%20ref%29))
  ;[1 1 1] Heal the player and then call the parent function
  (Effects|SpawnEmitteratLocation "/Game/ParticleSystems/ItemPickup/PE_HealthPickup.PE_HealthPickup" (Transformation|GetWorldLocation (Variables|Default|GetM_fish)))
  (Default|Heal PlayerWhoCollectedItem (Variables|Default|GetHealVal))
  (Development|PrintString "Healed")
  (|CallParentFunction PlayerWhoCollectedItem) ; This will call the parent pickup function and destroy the actor.
  (return ""))