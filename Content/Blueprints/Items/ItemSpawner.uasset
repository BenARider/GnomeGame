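; ItemSpawner periodically drops random pickups into the level.
; On BeginPlay it spawns an ItemSpawnArea at a hard-coded location, caches its center and world scale, and starts a looping timer.
; Each tick rolls spawn odds, then cascading re-rolls choose the item, placed at random XY within center ± scale.
; The Golden Shovel roll always passes, leaving Silver Bob and Spring Boots unreachable after Health Pack and Flaming Boots.
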(event Custom|ChanceToSpawnItem
  (bind _returnvalue (Math|Random|RandomInteger 99))
  (bind _itemspawnboxscale (Variables|Default|GetItemSpawnBoxScale))
  (bind _itemspawnlocationcenter (Variables|Default|GetItemSpawnLocationCenter))
  (bind _itemspawnboxscale_2 (Variables|Default|GetItemSpawnBoxScale))
  (bind _itemspawnlocationcenter_2 (Variables|Default|GetItemSpawnLocationCenter))
  (bind _y (Math|Vector|BreakVector _itemspawnboxscale))
  (bind _y_2 (Math|Vector|BreakVector _itemspawnlocationcenter_2))
  (bind (_x _y_3 _z) (Math|Vector|BreakVector _itemspawnboxscale_2))
  (bind (_x_2 _y_4 _z_2) (Math|Vector|BreakVector _itemspawnlocationcenter))
  ;[1 1 1] Spawn Items
  (if (== 0 (Math|Random|RandomInteger (Variables|Default|GetoddsOfSpawning)))
    (if (< _returnvalue 1) ; Health Pack
      (Variables|Default|SetitemToSpawn "/Game/Blueprints/Items/HealthPack.HealthPack_C")
      (Development|PrintString "Health Pack Spwaned")
      (Game|SpawnActorfromClass (Variables|Default|GetitemToSpawn) (Math|Transform|MakeTransform (Math|Vector|MakeVector (Math|Random|RandomFloatinRange (- _x_2 _x) (+ _x_2 _x)) (Math|Random|RandomFloatinRange (- _y_2 _y) (+ _y_2 _y)) (+ _z_2 _z))) "Undefined" 0 "NewEnumerator2" 0 :!label _label)
      (elif (< _returnvalue 2) ; Flaming Boots
        (Variables|Default|SetitemToSpawn "/Game/Blueprints/Items/FlamingBoots.FlamingBoots_C")
        (Development|PrintString "Boots Spawned")
        (goto _label)
        (elif (< _returnvalue 99) ; Golden Shovel
          (Variables|Default|SetitemToSpawn "/Game/Blueprints/Items/GoldenShovel.GoldenShovel_C")
          (Development|PrintString "Golden Shovel Spawned")
          (goto _label)
          (elif (< _returnvalue 80) ; Silver Bob
            (Variables|Default|SetitemToSpawn "/Game/Blueprints/Items/SilverBob.SilverBob_C")
            (Development|PrintString "Silver Bob Spawned")
            (goto _label)
            (elif (< _returnvalue 99) ; Spring
              (Variables|Default|SetitemToSpawn "/Game/Blueprints/Items/SpringBoots.SpringBoots_C")
              (Development|PrintString "Spring Boots Spawned")
              (goto _label)
              (else
                (Development|PrintString "Error with random int")))))))))

(event EventBeginPlay
  (bind _returnvalue (Game|SpawnActorfromClass "/Game/Blueprints/ItemSpawn/ItemSpawnArea.ItemSpawnArea_C" (Math|Transform|MakeTransform "-720.000000,-520.000000,290.000000") "Undefined" 0 0))
  (Variables|Default|SetItemSpawnLocationCenter (Transformation|GetActorLocation _returnvalue))
  (Variables|Default|SetItemSpawnBoxScale (Transformation|GetWorldScale (Variables|/Script/Engine.TriggerBase|GetCollisionComponent _returnvalue)))
  (Utilities|Time|SetTimerbyEvent (delegate Custom|ChanceToSpawnItem) (Variables|Default|GetitemSpawnTimer) true) ; Every certain number of seconds, do Spawn Items
)

(fn ConstructionScript)