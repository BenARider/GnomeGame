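; RoyaleRumble runs a local four-player gnome brawl, from lobby confirmation to the return to MainMenu.
; BeginPlay spawns gnomes at PlayerStarts, and confirm events toggle their visibility and active flags.
; StartGame destroys unconfirmed gnomes and starts the match timer plus looping checks that refresh CameraFix and count survivors.
; Dead gnomes stay hidden until a countdown respawns them, and the match ends on timeout or when at most one has lives left.
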(event Custom|CheckDelay
  (bind _isdead (Variables|Default|GetIsDead))
  (bind _delays (Variables|Default|GetDelays))
  (Variables|Default|SetAliveCount 0)
  (for _array_element (Variables|Default|GetPlayers)
    (Utilities|IsValid _array_element
      (:Is%20Valid
        (if (> (Variables|/Game/Blueprints/Gnome.Gnome_C|GetlivesRemaining _array_element) 0)
          (Math|Integer|IncrementInt (Variables|Default|GetAliveCount)
            (:%20%20
              (Variables|Default|SetWinnerID (Variables|/Game/Blueprints/Gnome.Gnome_C|GetPlayerID%20 _array_element))))))))
  (switch int (Variables|Default|GetAliveCount)
    (:Default
      (Variables|Default|SetWinnerID -1)
      (for (_array_element_2 _array_index) _isdead
        (if _array_element_2
          (if (> (Utilities|Array|Get(acopy) _delays _array_index) 0.0)
            (bind _result (Math|Float|DecrementFloat (Utilities|Array|Get(acopy) _delays _array_index))
              (:%20%20
                (Utilities|Array|SetArrayElem _delays _array_index _result)))
            (else
              (Utilities|Array|SetArrayElem _isdead _array_index false)
              (CallFunction|Respawn _array_index))))))
    (:0
      (Development|PrintString "tie")
      (CallFunction|GameEnd))
    (:1
      (Development|PrintString "Hello")
      (CallFunction|GameEnd))))

(event Custom|PlayerConfirmed
  (params (ID :type Integer))
  (if (not (Variables|Default|GetAllConfirmed))
    (CallFunction|ShowPlayer ID)
    (switch int ID
      (:0
        (Variables|Default|SetP1Active true))
      (:1
        (Variables|Default|SetP2Active true))
      (:2
        (Variables|Default|SetP3Active true))
      (:3
        (Variables|Default|SetP4Active true)))
    (bind _result (Math|Integer|IncrementInt (Variables|Default|GetPlayerCount))
      (:%20%20
        (Variables|Default|SetPlayerCount _result)))))

(event Custom|StartGame
  (if (not (Variables|Default|GetAllConfirmed))
    (if (> (Variables|Default|GetPlayerCount) 0)
      (Variables|Default|SetAllConfirmed true)
      (for _array_element (Variables|Default|GetPlayers)
        (bind _asgnome (Utilities|Casting|CastToGnome _array_element))
        (Utilities|IsValid _asgnome
          (:Is%20Valid
            (Variables|/Game/Blueprints/Gnome.Gnome_C|SethasStarted _asgnome true))
          (:Is%20Not%20Valid
            _))
        (CallFunction|CheckActivePlayers)
        (Utilities|Time|SetTimerbyFunctionName 0 "GameEnd" 1.8e+02)
        (Utilities|Time|SetTimerbyEvent (delegate Custom|CheckDelay) 1.0 true)
        (Utilities|Time|SetTimerbyEvent (delegate Custom|CheckCamera) 0.1 true)
        (bind _outactors (Actor|GetAllActorsOfClass "/Game/Blueprints/CameraFix.CameraFix_C"))
        (Default|Setup _outactors))
      (CallFunction|CheckActivePlayers)
      (Utilities|Time|SetTimerbyFunctionName 0 "GameEnd" 1.8e+02)
      (Utilities|Time|SetTimerbyEvent (delegate Custom|CheckDelay) 1.0 true)
      (Utilities|Time|SetTimerbyEvent (delegate Custom|CheckCamera) 0.1 true)
      (bind _outactors_2 (Actor|GetAllActorsOfClass "/Game/Blueprints/CameraFix.CameraFix_C"))
      (Default|Setup _outactors_2))))

(event Custom|PlayerUnconfirmed
  (params (ID :type Integer))
  (if (not (Variables|Default|GetAllConfirmed))
    (CallFunction|HidePlayer ID)
    (switch int ID
      (:0
        (Variables|Default|SetP1Active false))
      (:1
        (Variables|Default|SetP2Active false))
      (:2
        (Variables|Default|SetP3Active false))
      (:3
        (Variables|Default|SetP4Active false)))
    (bind _result (Math|Integer|DecrementInt (Variables|Default|GetPlayerCount))
      (:%20%20
        (Variables|Default|SetPlayerCount _result)))))

(event Custom|CheckCamera
  (bind _outactors (Actor|GetAllActorsOfClass "/Game/Blueprints/CameraFix.CameraFix_C"))
  (Default|Setup _outactors))

(event EventBeginPlay
  (Utilities|FlowControl|Sequence
    (:then_0
      (bind _returnvalue (UserInterface|CreateWidget "/Game/KingOfTheGarden/KotGUI.KotGUI_C"))
      (UserInterface|Viewport|AddtoViewport _returnvalue 100)
      (bind _outactors (Actor|GetAllActorsOfClass "/Script/Engine.PlayerStart"))
      (bind _output_get (Variables|Default|SetPlayerStartArray _outactors))
      (for (_array_element _array_index) _output_get
        (Utilities|Array|SetArrayElem (Variables|Default|GetSpawnPoints) _array_index (Transformation|GetActorTransform _array_element)))
      ;[1 1 1] Spawn Players
      (for (_ _array_index_2) (Variables|Default|GetPlayers)
        (Class|GameplayStatics|CreatePlayer _array_index_2)
        (Transformation|SetActorTransform (Game|Player|GetPlayerPawn _array_index_2) (Utilities|Array|Get(acopy) (Variables|Default|GetSpawnPoints) _array_index_2) false true)
        (bind _asgnome (Utilities|Casting|CastToGnome (Game|Player|GetPlayerPawn _array_index_2)))
        (Variables|/Game/Blueprints/Gnome.Gnome_C|SetPlayerID%20 _asgnome _array_index_2)
        (Utilities|Array|SetArrayElem (Variables|Default|GetPlayers) _array_index_2 _asgnome)
        (switch int _array_index_2
          (:0
            (Rendering|Material|SetMaterial (Variables|/Game/Blueprints/Gnome.Gnome_C|GetGnome_Rigged _asgnome) 0 "/Game/Meshs/Gnome/Textures/Clothes_MAT.Clothes_MAT")
            (Rendering|Material|SetMaterial (Variables|/Game/Blueprints/Gnome.Gnome_C|GetGnome_Rigged _asgnome) 1 "/Game/Meshs/Gnome/Textures/Hair_Mat.Hair_MAT"))
          (:1
            (Rendering|Material|SetMaterial (Variables|/Game/Blueprints/Gnome.Gnome_C|GetGnome_Rigged _asgnome) 0 "/Game/Materials/Gnome_2/Gnome_Low_Clothes_BaseColor_Mat.Gnome_Low_Clothes_BaseColor_Mat")
            (Rendering|Material|SetMaterial (Variables|/Game/Blueprints/Gnome.Gnome_C|GetGnome_Rigged _asgnome) 1 "/Game/Materials/Gnome_2/Gnome_Low_Hair_BaseColor_Mat.Gnome_Low_Hair_BaseColor_Mat"))
          (:2
            (Rendering|Material|SetMaterial (Variables|/Game/Blueprints/Gnome.Gnome_C|GetGnome_Rigged _asgnome) 0 "/Game/Materials/Gnome_3/Gnome_Low_Clothes_BaseColor_Mat.Gnome_Low_Clothes_BaseColor_Mat")
            (Rendering|Material|SetMaterial (Variables|/Game/Blueprints/Gnome.Gnome_C|GetGnome_Rigged _asgnome) 1 "/Game/Materials/Gnome_3/Gnome_Low_Hair_BaseColor_Mat.Gnome_Low_Hair_BaseColor_Mat"))
          (:3
            (Rendering|Material|SetMaterial (Variables|/Game/Blueprints/Gnome.Gnome_C|GetGnome_Rigged _asgnome) 0 "/Game/Materials/Gnome_4/Gnome_Low_Clothes_BaseColor_Mat.Gnome_Low_Clothes_BaseColor_Mat")
            (Rendering|Material|SetMaterial (Variables|/Game/Blueprints/Gnome.Gnome_C|GetGnome_Rigged _asgnome) 1 "/Game/Materials/Gnome_4/Gnome_Low_Hair_BaseColor_Mat.Gnome_Low_Hair_BaseColor_Mat"))))
      (CallFunction|HidePlayer 2)
      (CallFunction|HidePlayer 2)
      (CallFunction|HidePlayer 3))))

(fn ConstructionScript)

(fn GameEnd
  (Utilities|Time|SetTimerbyFunctionName 0 "OpenLevel2" 2.0))

(fn SpawnDelay
  (params (Player :type Gnome%20Object%20Reference))
  (bind _playerid_ (Variables|/Game/Blueprints/Gnome.Gnome_C|GetPlayerID%20 Player))
  (Utilities|Array|SetArrayElem (Variables|Default|GetDelays) _playerid_ 5.0)
  (Utilities|Array|SetArrayElem (Variables|Default|GetIsDead) _playerid_ true)
  (Rendering|SetActorHiddenInGame Player true))

(fn Respawn
  (params (ID :type Integer))
  (if (> (Variables|/Game/Blueprints/Gnome.Gnome_C|GetlivesRemaining (Utilities|Array|Get(acopy) (Variables|Default|GetPlayers) ID)) 0)
    (bind _asgnome (Utilities|Casting|CastToGnome (Utilities|Array|Get(acopy) (Variables|Default|GetPlayers) ID)))
    (Transformation|SetActorTransform _asgnome (Utilities|Array|Get(acopy) (Variables|Default|GetSpawnPoints) ID) false true)
    (Rendering|SetActorHiddenInGame _asgnome false)
    (Default|FullHeal _asgnome)
    (bind _outactors (Actor|GetAllActorsOfClass "/Game/Blueprints/CameraFix.CameraFix_C"))
    (Default|Setup _outactors)))

(fn HidePlayer
  (params (ID :type Integer))
  (Rendering|SetActorHiddenInGame (Utilities|Array|Get(acopy) (Variables|Default|GetPlayers) ID) true))

(fn ShowPlayer
  (params (ID :type Integer))
  (Rendering|SetActorHiddenInGame (Utilities|Array|Get(acopy) (Variables|Default|GetPlayers) ID) false))

(fn CheckActivePlayers
  (bind _players (Variables|Default|GetPlayers))
  (bind _output (Utilities|Array|Get(acopy) _players 3))
  (bind _output_2 (Utilities|Array|Get(acopy) _players))
  (bind _output_3 (Utilities|Array|Get(acopy) _players 1))
  (bind _output_4 (Utilities|Array|Get(acopy) _players 2))
  (if (Variables|Default|GetP1Active)
    _
    (elif (Utilities|IsValid _output_2)
      (Actor|DestroyActor _output_2)))
  (if (Variables|Default|GetP2Active)
    _
    (elif (Utilities|IsValid _output_3)
      (Actor|DestroyActor _output_3)))
  (if (Variables|Default|GetP3Active)
    _
    (elif (Utilities|IsValid _output_4)
      (Actor|DestroyActor _output_4)))
  (if (not (Variables|Default|GetP4Active))
    (if (Utilities|IsValid _output)
      (Actor|DestroyActor _output))))

(fn OpenLevel2
  (Game|OpenLevel(byName) "MainMenu"))