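; Spawner sets up local multiplayer at game start, creating a player per count, teleporting each Gnome pawn to its spawn point and storing it with a PlayerID.
; RespawnGnome deducts a life, then either destroys the Gnome or returns it to its ID's spawn point at full health.
; A looping one-second timer rolls a one-in-three item chance, which currently only prints a debug message.
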(event Custom|ChanceToSpawnItem
  ;[1 1 1] Spawn Items
  (if (== 0 (Math|Random|RandomInteger 3))
    (Development|PrintString "Item Spawned")))

(event EventBeginPlay
  ;[1 1 1] Spawn Gnomes when the game starts
  (Utilities|Time|SetTimerbyEvent (delegate Custom|ChanceToSpawnItem) 1.0 true)
  (while (< (Variables|Default|GetaddToPlayerArrayCounter) (Variables|Default|GetplayerCount)) ; While "Add to Player Array Counter" is less than player count.
    (Class|GameplayStatics|CreatePlayer (Variables|Default|GetaddToPlayerArrayCounter))
    (Transformation|SetActorTransform (Game|Player|GetPlayerPawn (Variables|Default|GetaddToPlayerArrayCounter)) (Utilities|Array|Get(acopy) (Variables|Default|GetSpawn%20Points) (Variables|Default|GetaddToPlayerArrayCounter)) false true)
    (bind _asgnome (Utilities|Casting|CastToGnome (Game|Player|GetPlayerPawn (Variables|Default|GetaddToPlayerArrayCounter))))
    (Variables|/Game/Blueprints/Gnome.Gnome_C|SetPlayerID%20 _asgnome (Variables|Default|GetaddToPlayerArrayCounter))
    (Utilities|Array|Add (Variables|Default|GetPlayers) _asgnome) ; Add the spawned gnome to an array for storage and future use. Might be a better idea to use a set or map using the PlayerID as a key instead of an array?
    (Variables|Default|SetaddToPlayerArrayCounter (+ (Variables|Default|GetaddToPlayerArrayCounter) 1)) ; Add to the counter.
  )
  (Development|PrintString (Utilities|String|ToString(Integer) (Utilities|Array|Length (Variables|Default|GetPlayers)))) ; On completion, print the amount in the array for debug purposes.
)

(fn ConstructionScript)

(fn RespawnGnome
  (params (Gnome :type Gnome%20Object%20Reference%20%28by%20ref%29))
  (bind _livesremaining (Variables|/Game/Blueprints/Gnome.Gnome_C|GetlivesRemaining Gnome))
  ;[1 1 1] Gnome Respawns if lives are above 0, otherwise is deleted
  (Development|PrintString "Has died")
  (Math|Integer|DecrementInt _livesremaining
    (:%20%20
      (if (<= _livesremaining 0)
        (Development|PrintString "No Lives Remaining")
        (Actor|DestroyActor Gnome)
        (else
          (Development|PrintString "Respawning")
          (bind _asgnome (Utilities|Casting|CastToGnome Gnome))
          (Transformation|SetActorTransform _asgnome (Utilities|Array|Get(acopy) (Variables|Default|GetSpawn%20Points) (Variables|/Game/Blueprints/Gnome.Gnome_C|GetPlayerID%20 _asgnome)) false true)
          (Default|FullHeal _asgnome))))))