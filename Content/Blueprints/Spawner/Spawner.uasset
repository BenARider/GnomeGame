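; Spawner manages local-multiplayer gnome players, their lives and random item drops.
; On BeginPlay it reads and destroys P1–P4 spawn markers, creates players with IDs, materials and a spawner reference, then runs CameraFix setup.
; A looping timer randomly drops one of five pickups via cascading rolls within a spawned ItemSpawnArea's bounds.
; RespawnGnome decrements lives, then teleports and heals the gnome, or destroys it and reruns camera setup.
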(event Custom|ChanceToSpawnItem
  (bind _returnvalue (Math|Random|RandomInteger 99))
  (bind _itemspawnboxscale (Variables|Default|GetItemSpawnBoxScale))
  (bind _itemspawnlocationcenter (Variables|Default|GetItemSpawnLocationCenter))
  (bind _itemspawnboxscale_2 (Variables|Default|GetItemSpawnBoxScale))
  (bind _itemspawnlocationcenter_2 (Variables|Default|GetItemSpawnLocationCenter))
  (bind _y (Math|Vector|BreakVector _itemspawnboxscale))
  (bind _y_2 (Math|Vector|BreakVector _itemspawnlocationcenter_2))
  (bind (_x _y_3 _z) (Math|Vector|BreakVector _itemspawnboxscale_2))
  (bind (_x_2 _y_4 _z_2) (Math|Vector|BreakVector _itemspawnlocationcenter))
  ;[1 1 1] Spawn Items
  (if (== 0 (Math|Random|RandomInteger (Variables|Default|GetoddsOfSpawning)))
    (if (< _returnvalue 20) ; Health Pack
      (Variables|Default|SetitemToSpawn "/Game/Blueprints/Items/HealthPack.HealthPack_C")
      (Development|PrintString "Health Pack Spwaned")
      (Game|SpawnActorfromClass (Variables|Default|GetitemToSpawn) (Math|Transform|MakeTransform (Math|Vector|MakeVector (Math|Random|RandomFloatinRange (- _x_2 _x) (+ _x_2 _x)) (Math|Random|RandomFloatinRange (- _y_2 _y) (+ _y_2 _y)) (+ _z_2 _z))) "Undefined" 0 "NewEnumerator2" 0 :!label _label)
      (elif (< _returnvalue 40) ; Flaming Boots
        (Variables|Default|SetitemToSpawn "/Game/Blueprints/Items/FlamingBoots.FlamingBoots_C")
        (Development|PrintString "Boots Spawned")
        (goto _label)
        (elif (< _returnvalue 60) ; Golden Shovel
          (Variables|Default|SetitemToSpawn "/Game/Blueprints/Items/GoldenShovel.GoldenShovel_C")
          (Development|PrintString "Golden Shovel Spawned")
          (goto _label)
          (elif (< _returnvalue 80) ; Silver Bob
            (Variables|Default|SetitemToSpawn "/Game/Blueprints/Items/SilverBob.SilverBob_C")
            (Development|PrintString "Silver Bob Spawned")
            (goto _label)
            (elif (< _returnvalue 99) ; Silver Bob
              (Variables|Default|SetitemToSpawn "/Game/Blueprints/Items/SpringBoots.SpringBoots_C")
              (Development|PrintString "Spring Boots Spawned")
              (goto _label)
              (else
                (Development|PrintString "Error with random int")))))))))

(event EventBeginPlay
  ;[1 1 1] Spawn Gnomes when the game starts
  (for (_ _array_index) (Variables|Default|GetSpawn%20Points)
    (switch int _array_index
      (:0
        (bind _outactors (Actor|GetAllActorsOfClass "/Game/Blueprints/Spawner/P1Spawn.P1Spawn_C"))
        (if (and (> (Utilities|Array|Length _outactors) 0) (< (Utilities|Array|Length _outactors) 2))
          (Utilities|Array|SetArrayElem (Variables|Default|GetSpawn%20Points) _array_index (Transformation|GetActorTransform (Utilities|Array|Get(acopy) _outactors)))
          (Actor|DestroyActor (Utilities|Array|Get(acopy) _outactors))
          (else
            (Development|PrintString "P1 either not there or has multiple. Using default values"))))
      (:1
        (bind _outactors_2 (Actor|GetAllActorsOfClass "/Game/Blueprints/Spawner/P2Spawn.P2Spawn_C"))
        (if (and (> (Utilities|Array|Length _outactors_2) 0) (< (Utilities|Array|Length _outactors_2) 2))
          (Utilities|Array|SetArrayElem (Variables|Default|GetSpawn%20Points) _array_index (Transformation|GetActorTransform (Utilities|Array|Get(acopy) _outactors_2)))
          (Actor|DestroyActor (Utilities|Array|Get(acopy) _outactors_2))
          (else
            (Development|PrintString "P2 either not there or has multiple. Using default values"))))
      (:2
        (bind _outactors_3 (Actor|GetAllActorsOfClass "/Game/Blueprints/Spawner/P3Spawn.P3Spawn_C"))
        (if (and (> (Utilities|Array|Length _outactors_3) 0) (< (Utilities|Array|Length _outactors_3) 2))
          (Utilities|Array|SetArrayElem (Variables|Default|GetSpawn%20Points) _array_index (Transformation|GetActorTransform (Utilities|Array|Get(acopy) _outactors_3)))
          (Actor|DestroyActor (Utilities|Array|Get(acopy) _outactors_3))
          (else
            (Development|PrintString "P3 either not there or has multiple. Using default values"))))
      (:3
        (bind _outactors_4 (Actor|GetAllActorsOfClass "/Game/Blueprints/Spawner/P4Spawn.P4Spawn_C"))
        (if (and (> (Utilities|Array|Length _outactors_4) 0) (< (Utilities|Array|Length _outactors_4) 2))
          (Utilities|Array|SetArrayElem (Variables|Default|GetSpawn%20Points) _array_index (Transformation|GetActorTransform (Utilities|Array|Get(acopy) _outactors_4)))
          (Actor|DestroyActor (Utilities|Array|Get(acopy) _outactors_4))
          (else
            (Development|PrintString "P4either not there or has multiple. Using default values"))))))
  (bind _returnvalue (Game|SpawnActorfromClass "/Game/Blueprints/ItemSpawn/ItemSpawnArea.ItemSpawnArea_C" (Math|Transform|MakeTransform "-720.000000,-520.000000,290.000000") "Undefined" 0 0))
  (Variables|Default|SetItemSpawnLocationCenter (Transformation|GetActorLocation _returnvalue))
  (Variables|Default|SetItemSpawnBoxScale (Transformation|GetWorldScale (Variables|/Script/Engine.TriggerBase|GetCollisionComponent _returnvalue)))
  (Utilities|Time|SetTimerbyEvent (delegate Custom|ChanceToSpawnItem) (Variables|Default|GetitemSpawnTimer) true) ; Every certain number of seconds, do Spawn Items
  (while (< (Variables|Default|GetaddToPlayerArrayCounter) (Variables|Default|GetplayerCount)) ; While "Add to Player Array Counter" is less than player count.
    (Class|GameplayStatics|CreatePlayer (Variables|Default|GetaddToPlayerArrayCounter))
    (Transformation|SetActorTransform (Game|Player|GetPlayerPawn (Variables|Default|GetaddToPlayerArrayCounter)) (Utilities|Array|Get(acopy) (Variables|Default|GetSpawn%20Points) (Variables|Default|GetaddToPlayerArrayCounter)) false true)
    (bind _asgnome (Utilities|Casting|CastToGnome (Game|Player|GetPlayerPawn (Variables|Default|GetaddToPlayerArrayCounter)))
      (:then
        (bind _output_get (Variables|/Game/Blueprints/Gnome.Gnome_C|SetPlayerID%20 _asgnome (Variables|Default|GetaddToPlayerArrayCounter)))
        (Utilities|Array|Add (Variables|Default|GetPlayers) _asgnome) ; Add the spawned gnome to an array for storage and future use. Might be a better idea to use a set or map using the PlayerID as a key instead of an array?
      )
      (:CastFailed
        _))
    (Variables|Default|SetaddToPlayerArrayCounter (+ (Variables|Default|GetaddToPlayerArrayCounter) 1)) ; Add to the counter.
    (Variables|/Game/Blueprints/Gnome.Gnome_C|SetSpawnerRef _asgnome self)
    (switch int _output_get
      (:0
        (Rendering|Material|SetMaterial (Variables|/Game/Blueprints/Gnome.Gnome_C|GetGnome_Rigged _asgnome) 0 "/Game/Meshs/Gnome/Textures/Clothes_MAT.Clothes_MAT")
        (Rendering|Material|SetMaterial (Variables|/Game/Blueprints/Gnome.Gnome_C|GetGnome_Rigged _asgnome) 1 "/Game/Meshs/Gnome/Textures/Hair_Mat.Hair_MAT"))
      (:1
        (Rendering|Material|SetMaterial (Variables|/Game/Blueprints/Gnome.Gnome_C|GetGnome_Rigged _asgnome) 0 "/Game/Materials/Gnome_2/Gnome_Low_Clothes_BaseColor_Mat.Gnome_Low_Clothes_BaseColor_Mat")
        (Rendering|Material|SetMaterial (Variables|/Game/Blueprints/Gnome.Gnome_C|GetGnome_Rigged _asgnome) 1 "/Game/Materials/Gnome_2/Gnome_Low_Hair_BaseColor_Mat.Gnome_Low_Hair_BaseColor_Mat"))
      (:2
        (Rendering|Material|SetMaterial (Variables|/Game/Blueprints/Gnome.Gnome_C|GetGnome_Rigged _asgnome) 0 "/Game/Materials/Gnome_3/Gnome_Low_Clothes_BaseColor_Mat.Gnome_Low_Clothes_BaseColor_Mat")
        (Rendering|Material|SetMaterial (Variables|/Game/Blueprints/Gnome.Gnome_C|GetGnome_Rigged _asgnome) 1 "/Game/Materials/Gnome_3/Gnome_Low_Hair_BaseColor_Mat.Gnome_Low_Hair_BaseColor_Mat"))
      (:3
        (Rendering|Material|SetMaterial (Variables|/Game/Blueprints/Gnome.Gnome_C|GetGnome_Rigged _asgnome) 0 "/Game/Materials/Gnome_4/Gnome_Low_Clothes_BaseColor_Mat.Gnome_Low_Clothes_BaseColor_Mat")
        (Rendering|Material|SetMaterial (Variables|/Game/Blueprints/Gnome.Gnome_C|GetGnome_Rigged _asgnome) 1 "/Game/Materials/Gnome_4/Gnome_Low_Hair_BaseColor_Mat.Gnome_Low_Hair_BaseColor_Mat"))))
  (Development|PrintString (Utilities|String|ToString(Integer) (Utilities|Array|Length (Variables|Default|GetPlayers)))) ; On completion, print the amount in the array for debug purposes.
  (bind _outactors_5 (Actor|GetAllActorsOfClass "/Game/Blueprints/CameraFix.CameraFix_C"))
  (Default|Setup _outactors_5))

(fn ConstructionScript)

(fn RespawnGnome
  (params (Gnome :type Gnome%20Object%20Reference%20%28by%20ref%29))
  (bind _capsule (Variables|/Game/Blueprints/Gnome.Gnome_C|GetCapsule Gnome))
  (bind _livesremaining (Variables|/Game/Blueprints/Gnome.Gnome_C|GetlivesRemaining Gnome))
  ;[1 1 1] Gnome Respawns if lives are above 0, otherwise is deleted
  (Physics|SetSimulatePhysics _capsule false)
  (Physics|SetSimulatePhysics _capsule true)
  (Development|PrintString "Has died")
  (Math|Integer|DecrementInt _livesremaining
    (:%20%20
      (if (<= _livesremaining 0)
        (Development|PrintString "No Lives Remaining")
        (Actor|DestroyActor Gnome)
        (bind _outactors (Actor|GetAllActorsOfClass "/Game/Blueprints/CameraFix.CameraFix_C"))
        (Default|Setup _outactors)
        (else
          (Development|PrintString "Respawning")
          (bind _asgnome (Utilities|Casting|CastToGnome Gnome))
          (Transformation|SetActorTransform _asgnome (Utilities|Array|Get(acopy) (Variables|Default|GetSpawn%20Points) (Variables|/Game/Blueprints/Gnome.Gnome_C|GetPlayerID%20 _asgnome)) false true)
          (Default|FullHeal _asgnome))))))